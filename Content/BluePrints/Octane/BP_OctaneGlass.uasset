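; BP_OctaneGlass is a glass cube that switches between solid and faded looks through two events, FadeGlass and BringGlass.
; Each event sets a transition material on the Cube, waits a fixed delay, then swaps in the matching end-state material.
; The Blueprint only swaps materials and does not change collision or visibility, leaving any animated transition to the materials themselves.
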(event Custom|FadeGlass
  (Rendering|Material|SetMaterial (Variables|Default|GetCube) 0 (Variables|Default|GetFadingGlass))
  (Utilities|FlowControl|Delay 3.0)
  (Rendering|Material|SetMaterial (Variables|Default|GetCube) 0 "/Game/Assets/Glass/MI_GlassFaded.MI_GlassFaded"))

(event Custom|BringGlass
  (Rendering|Material|SetMaterial (Variables|Default|GetCube) 0 (Variables|Default|GetGrowingGlass))
  (Utilities|FlowControl|Delay 3.0)
  (Rendering|Material|SetMaterial (Variables|Default|GetCube) 0 "/Game/StarterContent/Materials/M_Glass.M_Glass"))

(fn ConstructionScript)
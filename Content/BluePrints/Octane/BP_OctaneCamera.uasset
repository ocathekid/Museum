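; BP_OctaneCamera is a camera actor that blends the player's view to itself and back for an Octane display.
; GoToCamera takes the view and hides the BP_OctaneGlass cube.
; GoToPlayer blends to a given target, sets materials on BP_Octane's parts, removes all widgets and again hides the cube.
; BeginPlay caches BP_CameraSpline, but the interpolated spline-follow logic is disconnected and Tick is empty.
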(event Custom|GoToCamera
  ;[1 1 1] Moving to the camera, and then back to the player
  (Game|Player|SetViewTargetwithBlend (Game|GetPlayerController 0) self (Variables|Default|GetBlend%20Time) "VTBlend_Linear" 0.0 false)
  (bind _returnvalue (Actor|GetActorOfClass "/Game/BluePrints/Octane/BP_OctaneGlass.BP_OctaneGlass_C"))
  (Rendering|SetVisibility (Variables|/Game/BluePrints/Octane/BP_OctaneGlass.BP_OctaneGlass_C|GetCube _returnvalue) false false))

(event Custom|GoToPlayer
  (params (NewViewTarget :type Actor%20Object%20Reference))
  ;[1 1 1] Moving to the camera, and then back to the player
  (Game|Player|SetViewTargetwithBlend (Game|GetPlayerController 0) NewViewTarget (Variables|Default|GetBlend%20Time) "VTBlend_Linear" 0.0 false)
  (bind _returnvalue (Actor|GetActorOfClass "/Game/Assets/ArtPieces/Octane/BP_Octane.BP_Octane_C"))
  (Rendering|Material|SetMaterial (Variables|/Game/Assets/ArtPieces/Octane/BP_Octane.BP_Octane_C|GetOctane%20Body _returnvalue) 0 "/Game/Assets/ArtPieces/Octane/Body/Body.Body")
  (Rendering|Material|SetMaterial (Variables|/Game/Assets/ArtPieces/Octane/BP_Octane.BP_Octane_C|GetOctane%20Gear _returnvalue) 0 "/Game/Assets/ArtPieces/Octane/Gear/Gear.Gear")
  (Rendering|Material|SetMaterial (Variables|/Game/Assets/ArtPieces/Octane/BP_Octane.BP_Octane_C|GetOctane%20Camera _returnvalue) 0 "/Game/Assets/ArtPieces/Octane/Camera/Camera.Camera")
  (Rendering|Material|SetMaterial (Variables|/Game/Assets/ArtPieces/Octane/BP_Octane.BP_Octane_C|GetOctane%20Hands _returnvalue) 0 "/Game/Assets/ArtPieces/Octane/Hands/Hands.Hands")
  (Rendering|Material|SetMaterial (Variables|/Game/Assets/ArtPieces/Octane/BP_Octane.BP_Octane_C|GetOctane%20Head _returnvalue) 0 "/Game/Assets/ArtPieces/Octane/Head/Head.Head")
  (Rendering|Material|SetMaterial (Variables|/Game/Assets/ArtPieces/Octane/BP_Octane.BP_Octane_C|GetOctane%20JumpKit _returnvalue) 0 "/Game/Assets/ArtPieces/Octane/Jumpkit/Jumpkit.Jumpkit")
  (Viewport|RemoveAllWidgets)
  (Rendering|SetVisibility (Variables|/Game/BluePrints/Octane/BP_OctaneGlass.BP_OctaneGlass_C|GetCube (stale Custom|GoToCamera _returnvalue)) false false))

(event EventBeginPlay
  (bind _returnvalue (Actor|GetActorOfClass "/Game/BluePrints/Sword/BP_CameraSpline.BP_CameraSpline_C"))
  (Variables|Default|SetCameraSplineRef _returnvalue))

(event EventTick
  (params (DeltaSeconds :type Float%20%28single-precision%29))
  ;[1 1 1] Camera Moves Along Spline
)

(fn ConstructionScript)
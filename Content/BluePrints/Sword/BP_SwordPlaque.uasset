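; BP_SwordPlaque is an interactable plaque that opens a sword viewing mode.
; Overlapping its box adds a W_View widget, then enables input and the mouse cursor for the first-person character.
; Pressing V adds Sword_UI and calls GoToCamera on every BP_SwordCamera.
; Ending overlap removes all widgets and reverses input and cursor for the character; widget changes precede both character checks, so any overlapping actor triggers them.
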(event OnComponentBeginOverlap(Box)
  (params (OverlappedComponent :type Primitive%20Component%20Object%20Reference) (OtherActor :type Actor%20Object%20Reference) (OtherComp :type Primitive%20Component%20Object%20Reference) (OtherBodyIndex :type Integer) (bFromSweep :type Boolean) (SweepResult :type Hit%20Result%20Structure%20%28by%20ref%29))
  (bind _returnvalue (UserInterface|CreateWidget "/Game/Widgets/W_View.W_View_C"))
  (UserInterface|Viewport|AddtoViewport _returnvalue 0)
  (Utilities|Casting|CastToBP_FirstPersonCharacter OtherActor)
  (Input|EnableInput (Game|GetPlayerController 0))
  (Variables|/Script/Engine.PlayerController|SetbShowMouseCursor (Game|GetPlayerController 0) true))

(event EventBeginPlay)

(event Collision|EventActorBeginOverlap
  (params (OtherActor :type Actor%20Object%20Reference)))

(event EventTick
  (params (DeltaSeconds :type Float%20%28single-precision%29)))

(event Collision|EventActorEndOverlap
  (params (OtherActor :type Actor%20Object%20Reference))
  (Viewport|RemoveAllWidgets)
  (Utilities|Casting|CastToBP_FirstPersonCharacter (stale OnComponentBeginOverlap(Box) OtherActor))
  (Input|DisableInput (Game|GetPlayerController 0))
  (Variables|/Script/Engine.PlayerController|SetbShowMouseCursor (Game|GetPlayerController 0) false))

(event Input|KeyboardEvents|V
  (params (Key :type Key%20Structure :default "None"))
  (:Pressed
    (bind _returnvalue (UserInterface|CreateWidget "/Game/Assets/ArtPieces/Sword/Sword_UI.Sword_UI_C"))
    (UserInterface|Viewport|AddtoViewport _returnvalue 0)
    (bind _outactors (Actor|GetAllActorsOfClass "/Game/BluePrints/Sword/BP_SwordCamera.BP_SwordCamera_C"))
    (Default|GotoCamera _outactors)))

(fn ConstructionScript)
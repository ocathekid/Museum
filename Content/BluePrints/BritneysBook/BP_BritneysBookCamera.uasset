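; A camera actor for Britney's book that the player's view blends to and back from.
; GoToCamera blends the view to this actor and hides the book glass cube.
; GoToPlayer blends to a given target, restores the book's material, removes all widgets and shows the glass again.
; A spline reference is cached at BeginPlay, but the code moving the camera along it is disconnected and Tick is empty.
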(event Custom|GoToCamera
  ;[1 1 1] Moving to the camera, and then back to the player
  (Game|Player|SetViewTargetwithBlend (Game|GetPlayerController 0) self (Variables|Default|GetBlend%20Time) "VTBlend_Linear" 0.0 false)
  ;[1 1 1] Hiding Glass
  (bind _returnvalue (Actor|GetActorOfClass "/Game/BluePrints/BritneysBook/BP_BritneyBookGlass.BP_BritneyBookGlass_C"))
  (Rendering|SetVisibility (Variables|/Game/BluePrints/BritneysBook/BP_BritneyBookGlass.BP_BritneyBookGlass_C|GetCube _returnvalue) false false))

(event Custom|GoToPlayer
  (params (NewViewTarget :type Actor%20Object%20Reference))
  ;[1 1 1] Moving to the camera, and then back to the player
  (Game|Player|SetViewTargetwithBlend (Game|GetPlayerController 0) NewViewTarget (Variables|Default|GetBlend%20Time) "VTBlend_Linear" 0.0 false)
  ;[1 1 1] Setting model back to material
  (bind _returnvalue (Actor|GetActorOfClass "/Game/Assets/ArtPieces/Britney_Book/BP_BritneysBook.BP_BritneysBook_C"))
  (Rendering|Material|SetMaterial (Variables|/Game/Assets/ArtPieces/Britney_Book/BP_BritneysBook.BP_BritneysBook_C|GetBook_low _returnvalue) 0 "/Game/Assets/ArtPieces/Britney_Book/Materials/M_BritneysBook.M_BritneysBook")
  (Viewport|RemoveAllWidgets)
  (Rendering|SetVisibility (Variables|/Game/BluePrints/BritneysBook/BP_BritneyBookGlass.BP_BritneyBookGlass_C|GetCube (stale Custom|GoToCamera _returnvalue)) true false) ; Bringing glass back
)

(event EventBeginPlay
  (bind _returnvalue (Actor|GetActorOfClass "/Game/BluePrints/Sword/BP_CameraSpline.BP_CameraSpline_C"))
  (Variables|Default|SetCameraSplineRef _returnvalue))

(event EventTick
  (params (DeltaSeconds :type Float%20%28single-precision%29))
  ;[1 1 1] Camera Moves Along Spline
)

(fn ConstructionScript)
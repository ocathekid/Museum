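; BP_KateSwordPlaque is an interactable plaque for the Kate sword exhibit, using a box trigger and key input.
; Box overlap shows a W_View prompt, then enables input and the mouse cursor for the first-person character.
; V swaps the prompt for W_KateSword and moves to BP_KateSwordCamera's view; T calls its GoToPlayer to return.
; Ending overlap clears all widgets, then disables input and cursor for that character.
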(event OnComponentBeginOverlap(Box)
  (params (OverlappedComponent :type Primitive%20Component%20Object%20Reference) (OtherActor :type Actor%20Object%20Reference) (OtherComp :type Primitive%20Component%20Object%20Reference) (OtherBodyIndex :type Integer) (bFromSweep :type Boolean) (SweepResult :type Hit%20Result%20Structure%20%28by%20ref%29))
  (bind _returnvalue (UserInterface|CreateWidget "/Game/Widgets/W_View.W_View_C"))
  (bind _output_get (Variables|Default|SetViewWidget _returnvalue))
  (UserInterface|Viewport|AddtoViewport _output_get 0)
  (Utilities|Casting|CastToBP_FirstPersonCharacter OtherActor)
  (Input|EnableInput (Game|GetPlayerController 0))
  (Variables|/Script/Engine.PlayerController|SetbShowMouseCursor (Game|GetPlayerController 0) true))

(event EventBeginPlay)

(event Collision|EventActorBeginOverlap
  (params (OtherActor :type Actor%20Object%20Reference)))

(event EventTick
  (params (DeltaSeconds :type Float%20%28single-precision%29)))

(event Collision|EventActorEndOverlap
  (params (OtherActor :type Actor%20Object%20Reference))
  (Viewport|RemoveAllWidgets)
  (Utilities|Casting|CastToBP_FirstPersonCharacter (stale OnComponentBeginOverlap(Box) OtherActor))
  (Input|DisableInput (Game|GetPlayerController 0))
  (Variables|/Script/Engine.PlayerController|SetbShowMouseCursor (Game|GetPlayerController 0) false))

(event Input|KeyboardEvents|V
  (params (Key :type Key%20Structure :default "None"))
  (:Pressed
    (bind _returnvalue (UserInterface|CreateWidget "/Game/Widgets/W_KateSword.W_KateSword_C"))
    (UserInterface|Viewport|AddtoViewport _returnvalue 0)
    (Widget|RemovefromParent (Variables|Default|GetViewWidget))
    (bind _returnvalue_2 (Actor|GetActorOfClass "/Game/BluePrints/KateSword/BP_KateSwordCamera.BP_KateSwordCamera_C"))
    (Default|GotoCamera _returnvalue_2)))

(event Input|KeyboardEvents|T
  (params (Key :type Key%20Structure :default "None"))
  (:Pressed
    (Input|EnableInput (Game|GetPlayerController 0))
    (bind _returnvalue (Actor|GetActorOfClass "/Game/BluePrints/KateSword/BP_KateSwordCamera.BP_KateSwordCamera_C"))
    (Default|GotoPlayer _returnvalue (stale OnComponentBeginOverlap(Box) OtherActor))))

(fn ConstructionScript)
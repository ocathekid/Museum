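; BP_KateSwordCamera is a camera actor that takes over the player's view and hands it back.
; GoToCamera blends the player controller's view to this actor; GoToPlayer blends to a given target, resets the Sword_BP blade material to M_Sword and removes all widgets.
; BeginPlay caches a BP_CameraSpline reference, but the interpolated spline-following logic is disconnected from the empty Tick, so the camera never moves along it.
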(event Custom|GoToCamera
  ;[1 1 1] Moving to the camera, and then back to the player
  (Game|Player|SetViewTargetwithBlend (Game|GetPlayerController 0) self (Variables|Default|GetBlend%20Time) "VTBlend_Linear" 0.0 false))

(event Custom|GoToPlayer
  (params (NewViewTarget :type Actor%20Object%20Reference))
  ;[1 1 1] Moving to the camera, and then back to the player
  (Game|Player|SetViewTargetwithBlend (Game|GetPlayerController 0) NewViewTarget (Variables|Default|GetBlend%20Time) "VTBlend_Linear" 0.0 false)
  (bind _returnvalue (Actor|GetActorOfClass "/Game/Assets/ArtPieces/Sword/Sword_BP.Sword_BP_C"))
  (Rendering|Material|SetMaterial (Variables|/Game/Assets/ArtPieces/Sword/Sword_BP.Sword_BP_C|GetSword _returnvalue) 0 "/Game/Assets/ArtPieces/Sword/Sword_Material/M_Sword.M_Sword")
  (Viewport|RemoveAllWidgets))

(event EventBeginPlay
  (bind _returnvalue (Actor|GetActorOfClass "/Game/BluePrints/Sword/BP_CameraSpline.BP_CameraSpline_C"))
  (Variables|Default|SetCameraSplineRef _returnvalue))

(event EventTick
  (params (DeltaSeconds :type Float%20%28single-precision%29))
  ;[1 1 1] Camera Moves Along Spline
)

(fn ConstructionScript)
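; TurnONOFF is a trigger actor that lets the first-person player switch on a car's headlights.
; Overlapping its Box shows the W_View widget, and for the player enables input and the cursor; leaving removes all widgets and reverses both.
; Pressing V plays the Opacity timeline forward, driving both spotlights' intensity and applying the headlight glass material to two Car meshes, with no switch-off path.
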(event OnComponentBeginOverlap(Box)
  (params (OverlappedComponent :type Primitive%20Component%20Object%20Reference) (OtherActor :type Actor%20Object%20Reference) (OtherComp :type Primitive%20Component%20Object%20Reference) (OtherBodyIndex :type Integer) (bFromSweep :type Boolean) (SweepResult :type Hit%20Result%20Structure%20%28by%20ref%29))
  (bind _returnvalue (UserInterface|CreateWidget "/Game/Widgets/W_View.W_View_C"))
  (bind _output_get (Variables|Default|SetViewWidget _returnvalue))
  (UserInterface|Viewport|AddtoViewport _output_get 0)
  (Utilities|Casting|CastToBP_FirstPersonCharacter OtherActor)
  (Input|EnableInput (Game|GetPlayerController 0))
  (Variables|/Script/Engine.PlayerController|SetbShowMouseCursor (Game|GetPlayerController 0) true))

(event EventBeginPlay)

(event Collision|EventActorBeginOverlap
  (params (OtherActor :type Actor%20Object%20Reference)))

(event EventTick
  (params (DeltaSeconds :type Float%20%28single-precision%29)))

(event Collision|EventActorEndOverlap
  (params (OtherActor :type Actor%20Object%20Reference))
  (Viewport|RemoveAllWidgets)
  (Utilities|Casting|CastToBP_FirstPersonCharacter (stale OnComponentBeginOverlap(Box) OtherActor))
  (Input|DisableInput (Game|GetPlayerController 0))
  (Variables|/Script/Engine.PlayerController|SetbShowMouseCursor (Game|GetPlayerController 0) false))

(event Input|KeyboardEvents|V
  (params (Key :type Key%20Structure :default "None"))
  (:Pressed
    (bind _newtrack_0 (Timeline|Opacity Play)
      (:Update
        (Rendering|Components|Light|SetIntensity (Variables|Default|GetSpotLight1) _newtrack_0)
        (bind _returnvalue (Actor|GetActorOfClass "/Game/Assets/ArtPieces/Car/Car.Car_C"))
        (Rendering|Material|SetMaterial (Variables|/Game/Assets/ArtPieces/Car/Car.Car_C|GetCar_Big_HeadLigths _returnvalue) 0 "/Game/Assets/ArtPieces/Car/M_Glass_Headlights.M_Glass_Headlights")))))

(fn ConstructionScript)